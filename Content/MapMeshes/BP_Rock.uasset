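; BP_Rock is a map rock hazard that kills the player character on contact.
; When its static mesh hits a BP_JobaCharacter, it calls PlayerDead on that character.
; Two custom events, SimulatePhysics and StopPhysics, switch physics simulation on the mesh on and off.
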(event `self.StaticMesh.OnComponentHit`
  (params (HitComponent :type "PrimitiveComponent Object Reference") (OtherActor :type "Actor Object Reference") (OtherComp :type "PrimitiveComponent Object Reference") (NormalImpulse :type "Vector Structure") (Hit :type "HitResult Structure (by ref)"))
  (bind _asbp_joba_character (cast `/Game/Сharacter/BP_JobaCharacter` OtherActor))
  (`/Game/Сharacter/BP_JobaCharacter.PlayerDead` _asbp_joba_character))

(event `SimulatePhysics`
  (`PrimitiveComponent.SetSimulatePhysics` (`self.StaticMesh`) true))

(event `StopPhysics`
  (`PrimitiveComponent.SetSimulatePhysics` (`self.StaticMesh`) false))

(fn `UserConstructionScript`
  (`parent.UserConstructionScript`))