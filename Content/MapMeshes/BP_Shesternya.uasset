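; BP_Shesternya is a gear map object (the name is Russian for gear) that can be removed from play and restored.
; StartLogic hides its static mesh in game and disables collision, while RestartObject shows it again with query and physics collision.
; The actor stays in the world rather than being destroyed, and BeginPlay, overlap and Tick carry no active logic.
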(event `self.StartLogic`
  (bind _staticmesh (`self.StaticMesh`))
  (`SceneComponent.SetHiddenInGame` _staticmesh true false)
  (`PrimitiveComponent.SetCollisionEnabled` _staticmesh "NoCollision"))

(event `self.RestartObject`
  (bind _staticmesh (`self.StaticMesh`))
  (`SceneComponent.SetHiddenInGame` _staticmesh false false)
  (`PrimitiveComponent.SetCollisionEnabled` _staticmesh "QueryAndPhysics"))

(fn `UserConstructionScript`
  (`parent.UserConstructionScript`))