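; BP_SwitchebleObject is a map object that changes between a normal-world and a parallel-world version.
; Its LogicSwitch event, bound to the player character's universe-switch event on BeginPlay, swaps the static mesh, material and relative transform.
; The construction script applies the same swap from IsInParallelWorld, while BeginPlay starts the object in the normal state.
; A Box overlap clears the character's CanUseParaller while inside and restores it on exit.
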(event `self.ReceiveBeginPlay`
  (`self.LogicSwitch` false)
  (bind _asbp_joba_character (cast `/Game/Сharacter/BP_JobaCharacter` (`GameplayStatics.GetPlayerCharacter` 0)))
  (bind _output_get (set `self.MainCharacter` _asbp_joba_character))
  (add `/Game/Сharacter/BP_JobaCharacter.UniverseSwitch` _output_get (delegate `LogicSwitch`)))

(event `LogicSwitch`
  (params (IsInParallelWorld :type Boolean))
  (bind _staticmesh (`self.StaticMesh`))
  (bind _output_get (set `self.IsInParallelWorld` IsInParallelWorld))
  (if _output_get
    (`StaticMeshComponent.SetStaticMesh` _staticmesh (`self.ParallerMesh`))
    (`PrimitiveComponent.SetMaterial` _staticmesh 0 (`self.ParallelMat`))
    (`SceneComponent.K2_SetRelativeTransform` (`self.StaticMesh`) (`self.ParallelTransform`) false false)
    (else
      (`StaticMeshComponent.SetStaticMesh` _staticmesh (`self.NormalMesh`))
      (`PrimitiveComponent.SetMaterial` _staticmesh 0 (`self.NormalMat`))
      (`SceneComponent.K2_SetRelativeTransform` (`self.StaticMesh`) (`self.NormalTransform`) false false))))

(event `StartLogic`
  (`KismetSystemLibrary.PrintString` (`KismetSystemLibrary.GetObjectName` self)))

(event `self.Box.OnComponentBeginOverlap`
  (params (OverlappedComponent :type "PrimitiveComponent Object Reference") (OtherActor :type "Actor Object Reference") (OtherComp :type "PrimitiveComponent Object Reference") (OtherBodyIndex :type Integer) (bFromSweep :type Boolean) (SweepResult :type "HitResult Structure (by ref)"))
  (bind _asbp_joba_character (cast `/Game/Сharacter/BP_JobaCharacter` OtherActor))
  (set `/Game/Сharacter/BP_JobaCharacter.CanUseParaller` false _asbp_joba_character))

(event `self.Box.OnComponentEndOverlap`
  (params (OverlappedComponent :type "PrimitiveComponent Object Reference") (OtherActor :type "Actor Object Reference") (OtherComp :type "PrimitiveComponent Object Reference") (OtherBodyIndex :type Integer))
  (bind _asbp_joba_character (cast `/Game/Сharacter/BP_JobaCharacter` OtherActor))
  (set `/Game/Сharacter/BP_JobaCharacter.CanUseParaller` true _asbp_joba_character))

(event `RestartObject`)

(fn `UserConstructionScript`
  (if (`self.IsInParallelWorld`)
    (`StaticMeshComponent.SetStaticMesh` (`self.StaticMesh`) (`self.ParallerMesh`))
    (`PrimitiveComponent.SetMaterial` (`self.StaticMesh`) 0 (`self.ParallelMat`))
    (`SceneComponent.K2_SetRelativeTransform` (`self.StaticMesh`) (`self.ParallelTransform`) false false)
    (else
      (`StaticMeshComponent.SetStaticMesh` (`self.StaticMesh`) (`self.NormalMesh`))
      (`PrimitiveComponent.SetMaterial` (`self.StaticMesh`) 0 (`self.NormalMat`))
      (`SceneComponent.K2_SetRelativeTransform` (`self.StaticMesh`) (`self.NormalTransform`) false false))))