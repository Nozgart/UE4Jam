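; BP_RockMyst is a map mystery trigger that spawns an enemy when the player touches it in the parallel world.
; Its Box overlap and hit events share one path that casts to BP_JobaCharacter and checks IsInParallelWorld.
; On success it spawns BP_JobaEnemy1 at SpawnLocation and calls UseClock on the character, with no guard against repeat triggers.
; StartRestart is left empty.
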(event `self.ReceiveBeginPlay`
  (`parent.ReceiveBeginPlay`))

(event `self.Box.OnComponentBeginOverlap`
  (params (OverlappedComponent :type "PrimitiveComponent Object Reference") (OtherActor :type "Actor Object Reference") (OtherComp :type "PrimitiveComponent Object Reference") (OtherBodyIndex :type Integer) (bFromSweep :type Boolean) (SweepResult :type "HitResult Structure (by ref)"))
  (bind _asbp_joba_character (cast `/Game/Сharacter/BP_JobaCharacter` OtherActor :!label _label))
  (if (`/Game/Сharacter/BP_JobaCharacter.IsInParallelWorld` _asbp_joba_character)
    (`|SpawnActorFromClass` "/Game/Enemy/BP_JobaEnemy1.BP_JobaEnemy1_C" (`KismetMathLibrary.Conv_VectorToTransform` (`self.SpawnLocation`)) "Undefined" "OverrideRootScale" null null)
    (`/Game/Сharacter/BP_JobaCharacter.UseClock` _asbp_joba_character)))

(event `self.Box.OnComponentHit`
  (params (HitComponent :type "PrimitiveComponent Object Reference") (OtherActor :type "Actor Object Reference") (OtherComp :type "PrimitiveComponent Object Reference") (NormalImpulse :type "Vector Structure") (Hit :type "HitResult Structure (by ref)"))
  (goto _label))

(event `self.StartRestart`)

(fn `UserConstructionScript`
  (`parent.UserConstructionScript`))