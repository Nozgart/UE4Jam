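; Lift actor for a map that stays locked until the player's BP_JobaCharacter brings a key to its button.
; StartLogic branches on the hit component's tag: the button reveals and animates into place, zeroes the key count and enables the lift.
; The lift mesh then alternates up and down via a FlipFlop-driven timeline lerp.
; StartRestart restarts the linked key, disables the lift and resets its position, but leaves the button's DoOnce untouched.
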(event `self.StartLogic`
  (params (HitComponent :type "PrimitiveComponent Object Reference"))
  (switch `name` (`|GetArrayItem` (`ActorComponent.ComponentTags` HitComponent))
    (:`UpMesh`
      (if (`self.CanLift`)
        (`/Engine/EditorBlueprintResources/StandardMacros.FlipFlop`
          (:`A`
            (bind (_direction _newtrack_0) (`Timeline|Timeline_0` :!label _label)
              (:`Update`
                (`SceneComponent.K2_SetRelativeLocation` (`self.LiftMesh`) (`KismetMathLibrary.VLerp` (`self.FirstLocation`) (`self.SecondLocation`) _newtrack_0) false false))))
          (:`B`
            (goto _label :!via `Reverse`)))))
    (:`ButnMesh`
      (`/Engine/EditorBlueprintResources/StandardMacros.DoOnce` false :!label _label_2
        (:`Completed`
          (bind _asbp_joba_character (cast `/Game/Сharacter/BP_JobaCharacter` (`GameplayStatics.GetPlayerCharacter` 0)))
          (if (> (`/Game/Сharacter/BP_JobaCharacter.NumOfKeys` _asbp_joba_character) 0)
            (`SceneComponent.SetHiddenInGame` (`self.Butn`) false false)
            (bind (_direction_2 _newtrack_1) (`Timeline|AnimTM` :!via `PlayFromStart`)
              (:`Update`
                (`SceneComponent.K2_SetRelativeLocation` (`self.Butn`) (`KismetMathLibrary.VLerp` (`self.AnimFirst`) (`self.AnimSecond`) _newtrack_1) false false))
              (:`Finished`
                (set `/Game/Сharacter/BP_JobaCharacter.NumOfKeys` (- (`/Game/Сharacter/BP_JobaCharacter.NumOfKeys` _asbp_joba_character) (`/Game/Сharacter/BP_JobaCharacter.NumOfKeys` _asbp_joba_character)) _asbp_joba_character)
                (set `self.CanLift` true)
                (set `self.IsNeedToRestart` false)))
            (else
              (goto _label_2 :!via `Reset`))))))))

(event `self.StartRestart`
  (`/Game/MapMeshes/BP_SwitchebleObject.RestartObject` (`self.KeyToRestart`))
  (set `self.CanLift` false)
  (`SceneComponent.K2_SetRelativeLocation` (`self.LiftMesh`) (`self.LocationToReset`) false false))

(fn `UserConstructionScript`
  (bind _firstlocation (`self.FirstLocation`))
  (`parent.UserConstructionScript`)
  (set `self.LocationToReset` _firstlocation)
  (`SceneComponent.K2_SetRelativeLocation` (`self.LiftMesh`) _firstlocation false false)
  (`SceneComponent.K2_SetRelativeLocation` (`self.Butn`) (`self.AnimFirst`) false false))