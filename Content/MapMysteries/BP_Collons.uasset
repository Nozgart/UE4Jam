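; Map mystery puzzle where five columns must be triggered in order to reveal a hidden plane object.
; StartSpecificLogic reads the hit object's second tag, advances chained check flags with sound feedback, clears progress on out-of-order hits, and locks on completion.
; StartRestart clears the flags and hides the plane.
; The construction script sets column collision channels and passes normal and parallel meshes and materials to the plane's switchable child actor.
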(event `self.StartSpecificLogic`
  (params (HitObject :type "Actor Object Reference"))
  (if (`self.CanUse`)
    (switch `name` (`|GetArrayItem` (`Actor.Tags` HitObject) 1)
      (:`Column1`
        (set `self.IsFirstCheck` true)
        (`GameplayStatics.PlaySound2D` (`self.CorrectSound`)))
      (:`Column2`
        (if (`self.IsFirstCheck`)
          (set `self.IsSecondCheck` true)
          (`GameplayStatics.PlaySound2D` (`self.CorrectSound`))
          (else
            (set `self.IsFirstCheck` false)
            (`GameplayStatics.PlaySound2D` (`self.UncorrectSound`)))))
      (:`Column3`
        (if (and (`self.IsFirstCheck`) (`self.IsSecondCheck`))
          (set `self.IsThirdCheck` true)
          (`GameplayStatics.PlaySound2D` (`self.CorrectSound`))
          (else
            (set `self.IsFirstCheck` false)
            (set `self.IsSecondCheck` false)
            (`GameplayStatics.PlaySound2D` (`self.UncorrectSound`)))))
      (:`Column4`
        (if (and (`self.IsFirstCheck`) (`self.IsSecondCheck`) (`self.IsThirdCheck`))
          (set `self.IsFouthCheck` true)
          (`GameplayStatics.PlaySound2D` (`self.CorrectSound`))
          (else
            (set `self.IsFirstCheck` false)
            (set `self.IsSecondCheck` false)
            (set `self.IsThirdCheck` false)
            (`GameplayStatics.PlaySound2D` (`self.UncorrectSound`)))))
      (:`Column5`
        (if (and (`self.IsFirstCheck`) (`self.IsSecondCheck`) (`self.IsThirdCheck`) (`self.IsFouthCheck`))
          (set `self.IsFifthCheck` true)
          (set `self.IsNeedToRestart` false)
          (set `self.CanUse` false)
          (`SceneComponent.SetHiddenInGame` (`self.PlaneMesh`) false false)
          (`GameplayStatics.PlaySound2D` (`self.FinalSound`))
          (else
            (set `self.IsFirstCheck` false)
            (set `self.IsSecondCheck` false)
            (set `self.IsThirdCheck` false)
            (set `self.IsFouthCheck` false)
            (`GameplayStatics.PlaySound2D` (`self.UncorrectSound`))))))))

(event `self.StartLogic`
  (params (HitComponent :type "PrimitiveComponent Object Reference")))

(event `self.StartRestart`
  (set `self.IsFirstCheck` false)
  (set `self.IsSecondCheck` false)
  (set `self.IsThirdCheck` false)
  (set `self.IsFouthCheck` false)
  (set `self.IsFifthCheck` false)
  (`SceneComponent.SetHiddenInGame` (`self.PlaneMesh`) true false))

(fn `UserConstructionScript`
  (`parent.UserConstructionScript`)
  (`SceneComponent.K2_SetRelativeLocation` (`self.PlaneMesh`) (`self.PlaneLocation`) false false)
  (for _array_element (`|MakeArray` (`ChildActorComponent.ChildActor` (`self.Column1`)) (`ChildActorComponent.ChildActor` (`self.Column2`)) (`ChildActorComponent.ChildActor` (`self.Column3`)) (`ChildActorComponent.ChildActor` (`self.Column4`)) (`ChildActorComponent.ChildActor` (`self.Column5`)))
    (bind _asbp_switcheble_object (cast `/Game/MapMeshes/BP_SwitchebleObject` _array_element))
    (`PrimitiveComponent.SetCollisionObjectType` (`/Game/MapMeshes/BP_SwitchebleObject.StaticMesh` _asbp_switcheble_object) "ECC_GameTraceChannel2"))
  (bind _asbp_switcheble_object_2 (cast `/Game/MapMeshes/BP_SwitchebleObject` (`ChildActorComponent.ChildActor` (`self.PlaneMesh`))))
  (set `/Game/MapMeshes/BP_SwitchebleObject.NormalMesh` (`self.NormalMesh`) _asbp_switcheble_object_2)
  (set `/Game/MapMeshes/BP_SwitchebleObject.ParallerMesh` (`self.ParallelMesh`) _asbp_switcheble_object_2)
  (set `/Game/MapMeshes/BP_SwitchebleObject.NormalMat` (`self.NormalMat`) _asbp_switcheble_object_2)
  (set `/Game/MapMeshes/BP_SwitchebleObject.ParallelMat` (`self.ParallelMat`) _asbp_switcheble_object_2))