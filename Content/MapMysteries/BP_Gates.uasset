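; Key-operated double gate for a map puzzle that unlocks once the player has delivered three keys.
; StartLogic takes the keys from BP_JobaCharacter, reveals and slides in one button per accumulated key via timelines, then flip-flops the two leaves open or closed in mirrored yaw.
; StartRestart respawns the linked keys and returns the buttons, hidden, to locations cached in the Construction Script.
; Tick prints FirstPlayed as debug output.
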(event `FirstAnim`
  (bind _firstbutn (`self.FirstButn`))
  (if (not (`self.FirstPlayed`))
    (`SceneComponent.SetHiddenInGame` _firstbutn false false)
    (bind (_direction _newtrack_0) (`Timeline|First` :!via `PlayFromStart`)
      (:`Update`
        (`SceneComponent.K2_SetRelativeLocation` _firstbutn (`KismetMathLibrary.VLerp` (`SceneComponent.RelativeLocation` _firstbutn) (`self.FirstAnimLoc`) _newtrack_0) false false))
      (:`Finished`
        (set `self.FirstPlayed` true)))))

(event `SecondAnim`
  (bind _secondbutn (`self.SecondButn`))
  (if (not (`self.SecondPlayed`))
    (`SceneComponent.SetHiddenInGame` _secondbutn false false)
    (bind (_direction _newtrack_1) (`Timeline|Second` :!via `PlayFromStart`)
      (:`Update`
        (`SceneComponent.K2_SetRelativeLocation` _secondbutn (`KismetMathLibrary.VLerp` (`SceneComponent.RelativeLocation` _secondbutn) (`self.SecondAnimLoc`) _newtrack_1) false false))
      (:`Finished`
        (set `self.SecondPlayed` true)))))

(event `ThirdAnim`
  (bind _thirdbutn (`self.ThirdButn`))
  (if (not (`self.ThirdPlayed`))
    (`SceneComponent.SetHiddenInGame` _thirdbutn false false)
    (bind (_direction _newtrack_2) (`Timeline|Third` :!via `PlayFromStart`)
      (:`Update`
        (`SceneComponent.K2_SetRelativeLocation` _thirdbutn (`KismetMathLibrary.VLerp` (`SceneComponent.RelativeLocation` _thirdbutn) (`self.ThirdAnimLoc`) _newtrack_2) false false))
      (:`Finished`
        (set `self.ThirdPlayed` true)))))

(event `self.ReceiveTick`
  (params (DeltaSeconds :type "Float (single-precision)"))
  (`parent.ReceiveTick` DeltaSeconds)
  (`KismetSystemLibrary.PrintString` (`KismetStringLibrary.Conv_BoolToString` (`self.FirstPlayed`)) true false (struct :`R` 0.296138 :`G` 0.000304 :`B` 0.000304 :`A` 1.0) 0.0))

(event `self.StartLogic`
  (params (HitComponent :type "PrimitiveComponent Object Reference"))
  (`|ExecutionSequence`
    (:`then_0`
      (bind _asbp_joba_character (cast `/Game/Сharacter/BP_JobaCharacter` (`GameplayStatics.GetPlayerCharacter` 0)))
      (bind _numofkeys (`/Game/Сharacter/BP_JobaCharacter.NumOfKeys` _asbp_joba_character))
      (if (> _numofkeys 0)
        (bind _output_get (set `self.KeysCount` (+ (`self.KeysCount`) _numofkeys)))
        (set `/Game/Сharacter/BP_JobaCharacter.NumOfKeys` (- (`/Game/Сharacter/BP_JobaCharacter.NumOfKeys` _asbp_joba_character) (`/Game/Сharacter/BP_JobaCharacter.NumOfKeys` _asbp_joba_character)) _asbp_joba_character)
        (switch `int` _output_get
          (:`1`
            (`self.FirstAnim`))
          (:`2`
            (`self.FirstAnim`)
            (`self.SecondAnim`))
          (:`3`
            (`self.FirstAnim`)
            (`self.SecondAnim`)
            (`self.ThirdAnim`)
            (set `self.KeysCount` 0)
            (set `self.CanLift` true)
            (set `self.IsNeedToRestart` false)))))
    (:`then_1`
      (if (`self.CanLift`)
        (`/Engine/EditorBlueprintResources/StandardMacros.FlipFlop`
          (:`A`
            (bind (_direction _newtrack_0) (`Timeline|Timeline_0` :!label _label)
              (:`Update`
                (bind (_returnvalue_roll _returnvalue_pitch _returnvalue_yaw) (`KismetMathLibrary.BreakRotator` (`KismetMathLibrary.RLerp` (struct) (struct :`Yaw` 90.0) _newtrack_0)))
                (`SceneComponent.K2_SetRelativeRotation` (`self.Scene1`) (`KismetMathLibrary.MakeRotator` 0.0 0.0 _returnvalue_yaw) false false)
                (`SceneComponent.K2_SetRelativeRotation` (`self.Scene`) (`KismetMathLibrary.MakeRotator` 0.0 0.0 (* _returnvalue_yaw -1.0)) false false))))
          (:`B`
            (goto _label :!via `Reverse`)))))))

(event `self.StartRestart`
  (bind _firstbutn (`self.FirstButn`))
  (bind _secondbutn (`self.SecondButn`))
  (bind _thirdbutn (`self.ThirdButn`))
  (for _array_element (`self.KeyToRespawn`)
    (`/Game/MapMeshes/BP_SwitchebleObject.RestartObject` _array_element))
  (set `self.KeysCount` 0)
  (set `self.FirstPlayed` false)
  (set `self.SecondPlayed` false)
  (set `self.ThirdPlayed` false)
  (`SceneComponent.SetHiddenInGame` _firstbutn true false)
  (`SceneComponent.K2_SetWorldLocation` _firstbutn (`self.FirstResetLoc`) false false)
  (`SceneComponent.SetHiddenInGame` _secondbutn true false)
  (`SceneComponent.K2_SetWorldLocation` _secondbutn (`self.SecondResetLoc`) false false)
  (`SceneComponent.SetHiddenInGame` _thirdbutn true false)
  (`SceneComponent.K2_SetWorldLocation` _thirdbutn (`self.ThirdResetLoc`) false false))

(fn `UserConstructionScript`
  (`parent.UserConstructionScript`)
  (set `self.FirstResetLoc` (`SceneComponent.K2_GetComponentLocation` (`self.FirstButn`)))
  (set `self.SecondResetLoc` (`SceneComponent.K2_GetComponentLocation` (`self.SecondButn`)))
  (set `self.ThirdResetLoc` (`SceneComponent.K2_GetComponentLocation` (`self.ThirdButn`))))