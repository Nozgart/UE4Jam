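; BP_JobaEnemy1 is an enemy that changes form and speed with the parallel world state.
; LogicSwitch stops movement, then either sets a fast monster with the Idle mesh, MonstrAnim and StartChase on, or a slow SkeletalCube with chasing off.
; StartChase is only set here, with no chase logic in this graph.
; The code binding LogicSwitch to BP_JobaCharacter's universe switch is disconnected and never runs.
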(event `LogicSwitch`
  (params (IsInParallelWorld :type Boolean))
  (bind _charactermovement (`self.CharacterMovement`))
  (bind _mesh (`self.Mesh`))
  (bind _charactermovement_2 (`self.CharacterMovement`))
  (bind _output_get (set `self.IsInParallelWorld` IsInParallelWorld))
  (if _output_get
    (`MovementComponent.StopMovementImmediately` _charactermovement)
    (set `CharacterMovementComponent.MaxWalkSpeed` 400.0 _charactermovement)
    (`SkinnedMeshComponent.SetSkinnedAssetAndUpdate` _mesh "/Game/Enemy/Mesh/Idle.Idle" false)
    (`SkeletalMeshComponent.SetAnimInstanceClass` _mesh "/Game/Enemy/Mesh/MonstrAnim.MonstrAnim_C")
    (set `self.StartChase` true)
    (else
      (set `self.StartChase` false)
      (`MovementComponent.StopMovementImmediately` _charactermovement_2)
      (set `CharacterMovementComponent.MaxWalkSpeed` 25.0 _charactermovement_2)
      (`SkinnedMeshComponent.SetSkinnedAssetAndUpdate` (`self.Mesh`) "/Engine/EngineMeshes/SkeletalCube.SkeletalCube" false))))

(fn `UserConstructionScript`)