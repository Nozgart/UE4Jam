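; Enemy that reacts to the player's universe switch, chasing as a monster in the parallel world and posing as a cube in the normal one.
; A callback bound on BP_JobaCharacter swaps mesh and walk speed and toggles the chase.
; Tick runs AI MoveTo toward the player while chasing.
; Otherwise, when not recently rendered, it briefly enables teleporting to the player's Arrow1 in a delayed loop.
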(event `self.ReceiveBeginPlay`
  (bind _asbp_joba_character (cast `/Game/Сharacter/BP_JobaCharacter` (`GameplayStatics.GetPlayerCharacter` 0)))
  (bind _output_get (set `self.MainCharacter` _asbp_joba_character))
  (add `/Game/Сharacter/BP_JobaCharacter.UniverseSwitch` _output_get (delegate `LogicSwitch`)))

(event `LogicSwitch`
  (params (IsInParallelWorld :type Boolean))
  (bind _charactermovement (`self.CharacterMovement`))
  (bind _mesh (`self.Mesh`))
  (bind _charactermovement_2 (`self.CharacterMovement`))
  (bind _output_get (set `self.IsInParallelWorld` IsInParallelWorld))
  (if _output_get
    (`MovementComponent.StopMovementImmediately` _charactermovement)
    (set `CharacterMovementComponent.MaxWalkSpeed` 400.0 _charactermovement)
    (`SkinnedMeshComponent.SetSkinnedAssetAndUpdate` _mesh "/Game/Enemy/Mesh/Idle.Idle" false)
    (`SkeletalMeshComponent.SetAnimInstanceClass` _mesh "/Game/Enemy/Mesh/MonstrAnim.MonstrAnim_C")
    (set `self.StartChase` true)
    (else
      (set `self.StartChase` false)
      (`MovementComponent.StopMovementImmediately` _charactermovement_2)
      (set `CharacterMovementComponent.MaxWalkSpeed` 25.0 _charactermovement_2)
      (`SkinnedMeshComponent.SetSkinnedAssetAndUpdate` (`self.Mesh`) "/Engine/EngineMeshes/SkeletalCube.SkeletalCube" false))))

(event `self.ReceiveTick`
  (params (DeltaSeconds :type "Float (single-precision)"))
  (bind _returnvalue (`GameplayStatics.GetPlayerCharacter` 0))
  (`|ExecutionSequence`
    (:`then_0`
      (set `self.Character` (`SceneComponent.K2_GetComponentLocation` (`/Game/Сharacter/BP_JobaCharacter.Arrow1` (cast `/Game/Сharacter/BP_JobaCharacter` _returnvalue :!pure true))))
      (set `self.Distance to characcter` (`KismetMathLibrary.VSize` (- (`self.K2_GetActorLocation` _returnvalue) (`SceneComponent.K2_GetComponentLocation` (`self.CapsuleComponent`)))))
      (`KismetSystemLibrary.PrintString` (`KismetStringLibrary.Concat_StrStr` "Parrallel World" "  " (`KismetStringLibrary.Conv_BoolToString` (`self.IsInParallelWorld`))) true true (struct :`R` 0.287441 :`A` 1.0) 0.0)
      (if (`self.StartChase`)
        (`|AIMoveTo` self (0.0 0.0 0.0) (`GameplayStatics.GetPlayerCharacter` 0) 5.0 true)
        (else
          (if (`self.WasRecentlyRendered` 0.2) :!label _label
            _
            (elif (`self.IsInParallelWorld`)
              (set `self.CanTP` false)
              (else
                (set `self.CanTP` true)
                (`KismetSystemLibrary.Delay` 0.1)
                (set `self.CanTP` false)
                (`KismetSystemLibrary.Delay` 1.5)
                (goto _label)))))))
    (:`then_1`
      (if (`self.CanTP`)
        (`SceneComponent.K2_SetWorldLocation` (`self.CapsuleComponent`) (`self.Character`) false true)))))

(fn `UserConstructionScript`)