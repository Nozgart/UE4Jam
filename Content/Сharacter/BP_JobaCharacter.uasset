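; First-person player character that uses a clock to switch between the normal and parallel worlds, broadcasting the change and recoloring the directional light.
; A per-tick sphere trace, with object types chosen by world, shows a prompt and feeds interaction with mysteries, keys and collectables.
; It also handles crouching, jumping and landing shakes, with fatal falls returning to a checkpoint through Joba_GM.
; Sprint events are empty, leaving their speed logic disconnected.
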(event `self.ReceiveTick`
  (params (DeltaSeconds :type "Float (single-precision)"))
  (bind (_returnvalue_x _returnvalue_y _returnvalue_z) (`KismetMathLibrary.BreakVector` (`self.GetVelocity`)))
  (bind _camera (`self.Camera`))
  (bind _returnvalue (`SceneComponent.K2_GetComponentLocation` _camera))
  ;[1 1 1] Give a grandpa some space you little fuck
  (`self.StaminaUse` (`self.IsStaminaUse`))
  (`KismetSystemLibrary.PrintString` (`KismetStringLibrary.Conv_DoubleToString` _returnvalue_z) true false (struct :`R` 0.351533 :`G` 0.991102 :`B` 0.059511 :`A` 1.0) 0.0)
  (bind _outhit (`KismetSystemLibrary.SphereTraceSingleForObjects` _returnvalue (+ _returnvalue (* (`SceneComponent.GetForwardVector` _camera) 150.0)) 20.0 (`|MakeArray` "ObjectTypeQuery8" (select `bool` (`self.IsInParallelWorld`) :`false` "ObjectTypeQuery7" :`true` "ObjectTypeQuery8" :!type "EObjectTypeQuery Enum"))))
  (bind (_bblockinghit _binitialoverlap _time _distance _location _impactpoint _normal _impactnormal _physmat _hitactor _hitcomponent) (`GameplayStatics.BreakHitResult` _outhit))
  (if _bblockinghit
    (`/Engine/EditorBlueprintResources/StandardMacros.DoOnce` false :!label _label
      (:`Completed`
        (`SceneComponent.SetHiddenInGame` (`self.Widget`) false false)
        (set `self.HitActor` _hitactor)
        (set `self.HitComponent` _hitcomponent)
        (goto _label_2 :!via `Reset`)))
    (else
      (`/Engine/EditorBlueprintResources/StandardMacros.DoOnce` false :!label _label_2
        (:`Completed`
          (`SceneComponent.SetHiddenInGame` (`self.Widget`) true false)
          (set `self.HitActor` null)
          (set `self.HitComponent` null)
          (goto _label :!via `Reset`))))))

(event `InputAction|UseSceneItem`
  (params (Key :type "Key Structure"))
  (bind _hitactor (`self.HitActor`))
  ;[1 1 1] Iteractions
  (:`Pressed`
    (`/Engine/EditorBlueprintResources/StandardMacros.IsValid` _hitactor
      (:`Is Valid`
        (`self.SelectLogic` _hitactor (`self.HitComponent`))))))

(event `UseClock`
  (bind _uimain (`self.UiMain`))
  (bind _charactermovement (`self.CharacterMovement`))
  (bind _clock (`self.Clock`))
  (bind _arm (`self.Arm`))
  (bind _lightcomponent (`Light.LightComponent` (`self.DirectionalLight`)))
  ;[1 1 1] Iteractions
  (`/Engine/EditorBlueprintResources/StandardMacros.DoOnce` false :!label _label_3
    (:`Completed`
      (`SceneComponent.K2_SetRelativeRotation` (`self.Clock`) (struct :`Pitch` -9.0 :`Yaw` -6.0 :`Roll` 6.0) false false)
      (if (`NavMovementComponent.IsFalling` (`self.CharacterMovement`))
        (goto _label_3 :!via `Reset`)
        (elif (and (`self.CanUseParaller`) (not (`self.IsDead`)))
          (`GameplayStatics.PlaySound2D` "/Game/sound/ClickClock.ClickClock" 1.3)
          (if (`self.IsInParallelWorld`)
            (`SkeletalMeshComponent.PlayAnimation` _arm "/Game/Hands/ClickArm_Anim.ClickArm_Anim" false)
            (`SceneComponent.K2_SetRelativeRotation` (`self.Clock`) (struct :`Pitch` -48.0 :`Yaw` -112.0 :`Roll` -157.0) false false)
            (`SkeletalMeshComponent.PlayAnimation` _clock "/Game/Hands/Clock/InverseClock.InverseClock" false)
            (`KismetSystemLibrary.Delay` 0.5)
            (`/Game/Widgets/MainUi.PlayFadeAnim` _uimain)
            (`LightComponent.SetLightColor` _lightcomponent (struct :`R` 1.0 :`G` 1.0 :`B` 1.0 :`A` 1.0) true)
            (set `self.IsInParallelWorld` false)
            (else
              (`SkeletalMeshComponent.PlayAnimation` _arm "/Game/Hands/ClickArm_Anim.ClickArm_Anim" false)
              (`SceneComponent.K2_SetRelativeRotation` (`self.Clock`) (struct :`Pitch` -48.0 :`Yaw` -112.0 :`Roll` -157.0) false false)
              (`SkeletalMeshComponent.PlayAnimation` _clock "/Game/Hands/Clock/NormalClock_clock2_Arrow_Anim.NormalClock_clock2_Arrow_Anim" false)
              (`KismetSystemLibrary.Delay` 0.5)
              (`/Game/Widgets/MainUi.PlayFadeAnim` _uimain)
              (`LightComponent.SetLightColor` _lightcomponent (select `int` (`KismetMathLibrary.RandomIntegerInRange` 0 2) :`0` (struct :`R` 1.0 :`A` 1.0) :`1` (struct :`G` 1.0 :`A` 1.0) :`2` (struct :`B` 1.0 :`A` 1.0) :!type "LinearColor Structure") true)
              (set `self.IsInParallelWorld` true)))
          (`CharacterMovementComponent.SetMovementMode` _charactermovement "MOVE_Flying" 0)
          (set `self.CanWalk` false)
          (`KismetSystemLibrary.Delay` 0.2)
          (`CharacterMovementComponent.SetMovementMode` _charactermovement "MOVE_Walking" 0)
          (set `self.CanWalk` true)
          (`self.UniverseSwitch` (`self.IsInParallelWorld`))
          (`KismetSystemLibrary.Delay` 1.0)
          (`SkeletalMeshComponent.PlayAnimation` (`self.Arm`) "/Game/Hands/Idle.Idle" true)
          (`SceneComponent.K2_SetRelativeRotation` (`self.Clock`) (struct :`Pitch` -9.0 :`Yaw` -6.0 :`Roll` 6.0) false false)
          (goto _label_3 :!via `Reset`)
          (else
            (goto _label_3 :!via `Reset`)))))))

(event `self.ReceiveBeginPlay`
  (bind _arm (`self.Arm`))
  (bind _asjoba_gm (cast `/Game/Joba_GM` (`GameplayStatics.GetGameMode`)))
  (set `self.MyGameMode` _asjoba_gm)
  (`GameplayStatics.PlaySound2D` "/Game/sound/AmbienceBackgroundNormal2.AmbienceBackgroundNormal2")
  (`GameplayStatics.PlaySound2D` "/Game/sound/Birds.Birds")
  (`GameplayStatics.PlaySound2D` "/Game/sound/Ocean.Ocean" 0.1)
  (`KismetSystemLibrary.Delay` 3.5)
  (`SceneComponent.SetVisibility` (`self.ArmShowOff`) false false)
  (`SceneComponent.SetVisibility` (`self.ClockShowOff`) false false)
  (bind (_direction _camera _speed _arm_2) (`Timeline|Timeline_0` :!via `PlayFromStart`)
    (:`Update`
      (`|ExecutionSequence`
        (:`then_0`
          (`SceneComponent.K2_SetRelativeLocation` _arm (`KismetMathLibrary.MakeVector` 13.8 -32.919998 (.z _arm_2)) false true))
        (:`then_1`
          (`CameraComponent.SetFieldOfView` (`self.Camera`) _camera))
        (:`then_2`
          (set `CharacterMovementComponent.MaxWalkSpeed` _speed (`self.CharacterMovement`)))))
    (:`Finished`
      (`SceneComponent.K2_SetRelativeLocation` _arm (13.8 -32.919998 -54.0) false true))))

(event `InputAction|UseItem`
  (params (Key :type "Key Structure"))
  ;[1 1 1] Iteractions
  (:`Pressed`
    (`self.UseClock`)))

(event `InputAxis|MoveForward`
  (params (AxisValue :type "Float (single-precision)"))
  ;[1 1 1] Controls
  (if (and (`self.CanWalk`) (not (`self.IsDead`)))
    (`self.AddMovementInput` (`KismetMathLibrary.GetForwardVector` (`KismetMathLibrary.MakeRotator` 0.0 0.0 (.yaw (`self.GetControlRotation`)))) AxisValue)
    (if (== AxisValue 0.0)
      _
      (elif (not (`NavMovementComponent.IsFalling` (`self.CharacterMovement`)))
        (`GameplayStatics.PlayWorldCameraShake` (`self.SelectShake`) (`self.K2_GetActorLocation`) 0.0 500.0)))))

(event `InputAxis|MoveRight`
  (params (AxisValue :type "Float (single-precision)"))
  ;[1 1 1] Controls
  (if (and (`self.CanWalk`) (not (`self.IsDead`)))
    (`self.AddMovementInput` (`KismetMathLibrary.GetRightVector` (`KismetMathLibrary.MakeRotator` 0.0 0.0 (.yaw (`self.GetControlRotation`)))) AxisValue)
    (if (== AxisValue 0.0)
      _
      (elif (not (`NavMovementComponent.IsFalling` (`self.CharacterMovement`)))
        (`GameplayStatics.PlayWorldCameraShake` (`self.SelectShake`) (`self.K2_GetActorLocation`) 0.0 500.0)))))

(event `InputAxis|LookForward`
  (params (AxisValue :type "Float (single-precision)"))
  ;[1 1 1] Controls
  (`self.AddControllerPitchInput` AxisValue))

(event `InputAxis|LookRight`
  (params (AxisValue :type "Float (single-precision)"))
  ;[1 1 1] Controls
  (`self.AddControllerYawInput` AxisValue))

(event `InputAction|CrouchAction`
  (params (Key :type "Key Structure"))
  (:`Pressed`
    (if (not (`self.IsDead`))
      (`self.SitDown`))))

(event `SitDown`
  (bind _charactermovement (`self.CharacterMovement`))
  (`/Engine/EditorBlueprintResources/StandardMacros.DoOnce` false :!label _label_4
    (:`Completed`
      (if (`self.IsCrouch`)
        (set `self.IsCrouch` false)
        (set `CharacterMovementComponent.MaxWalkSpeed` 300.0 _charactermovement)
        (bind (_direction _anim) (`Timeline|Crouch_TimeLine` :!via `ReverseFromEnd` :!label _label_5)
          (:`Update`
            (`CapsuleComponent.SetCapsuleHalfHeight` (`self.CapsuleComponent`) (`KismetMathLibrary.Lerp` 88.0 55.0 _anim) true)
            (`SceneComponent.K2_SetRelativeLocation` (`self.Camera`) (`KismetMathLibrary.MakeVector` 0.0 0.0 (`KismetMathLibrary.Lerp` 60.0 20.0 _anim)) false false))
          (:`Finished`
            (goto _label_4 :!via `Reset`)))
        (else
          (set `self.IsCrouch` true)
          (`self.StopRun`)
          (set `CharacterMovementComponent.MaxWalkSpeed` 100.0 _charactermovement)
          (goto _label_5))))))

(event `InputAction|SpeedRun`
  (params (Key :type "Key Structure"))
  (bind _iscrouch (`self.IsCrouch`))
  (:`Pressed`
    (if (not _iscrouch)
      (`self.StartRun`)))
  (:`Released`
    (if (not _iscrouch)
      (`self.StopRun`))))

(event `StartRun`)

(event `StopRun`)

(event `InputAction|JumpButton`
  (params (Key :type "Key Structure"))
  (:`Pressed`
    (if (not (`self.IsCrouch`))
      (`self.Jump`))))

(event `self.OnLanded`
  (params (Hit :type "HitResult Structure (by ref)"))
  (bind (_returnvalue_x _returnvalue_y _returnvalue_z) (`KismetMathLibrary.BreakVector` (`self.GetVelocity`)))
  (bind (_returnvalue_x_2 _returnvalue_y_2 _returnvalue_z_2) (`KismetMathLibrary.BreakVector` (`self.GetVelocity`)))
  (`self.StopJumping`)
  (if (<= _returnvalue_z_2 -1000.0)
    (set `self.IsDead` true)
    (`self.PlayerDead`)
    (elif (<= _returnvalue_z -750.0)
      (`GameplayStatics.PlayWorldCameraShake` "/Game/Сharacter/CameraShakes/HardLandedShake.HardLandedShake_C" (`self.K2_GetActorLocation`) 0.0 500.0)
      (else
        (`GameplayStatics.PlayWorldCameraShake` "/Game/Сharacter/CameraShakes/LandedShake.LandedShake_C" (`self.K2_GetActorLocation`) 0.0 500.0)))))

(event `PlayerDead`
  (set `self.IsDead` true)
  (`self.DeadScreen`))

(event `self.ReceivePossessed`
  (params (NewController :type "Controller Object Reference"))
  (set `self.CheckPointLocation` (`self.K2_GetActorLocation`))
  (`WidgetLayoutLibrary.RemoveAllWidgets`)
  (bind _returnvalue (`|CreateWidget` "/Game/Widgets/MainUi.MainUi_C"))
  (bind _output_get (set `self.UiMain` _returnvalue))
  (`UserWidget.AddToViewport` _output_get 0))

(event `self.ReceiveUnpossessed`
  (params (OldController :type "Controller Object Reference"))
  (`WidgetLayoutLibrary.RemoveAllWidgets`))

(event `self.ReceiveDestroyed`)

(event `SetNewCheckPoint`
  (params (CheckPointLocation :type "Vector Structure"))
  (set `self.CheckPointLocation` CheckPointLocation))

(event `Key|J`
  (params (Key :type "Key Structure")))

(event `DeadScreen`
  (if (`self.IsDead`)
    (bind _asjoba_gm (cast `/Game/Joba_GM` (`GameplayStatics.GetGameMode`)))
    (set `self.IsInParallelWorld` false)
    (`/Game/Widgets/MainUi.PlayFadeAnim` (`self.UiMain`))
    (`self.UniverseSwitch` (`self.IsInParallelWorld`))
    (`LightComponent.SetLightColor` (`Light.LightComponent` (`self.DirectionalLight`)) (struct :`R` 1.0 :`G` 1.0 :`B` 1.0 :`A` 1.0) true)
    (`/Game/Joba_GM.GoToCheckPoint` _asjoba_gm)))

(fn `SelectLogic`
  (params (HitActor :type "Actor Object Reference") (HitComponent :type "PrimitiveComponent Object Reference"))
  (bind _asbp_abstract_myst (cast `/Game/MapMysteries/BP_AbstractMyst` HitActor)
    (:`then`
      (`/Engine/EditorBlueprintResources/StandardMacros.IsValid` _asbp_abstract_myst
        (:`Is Valid`
          (`/Game/MapMysteries/BP_AbstractMyst.StartLogic` _asbp_abstract_myst HitComponent))))
    (:`CastFailed`
      (bind _asbp_switcheble_object (cast `/Game/MapMeshes/BP_SwitchebleObject` HitActor))
      (`|ExecutionSequence`
        (:`then_0`
          (switch `name` (`|GetArrayItem` (`Actor.Tags` _asbp_switcheble_object))
            (:`KeyObject`
              (set `self.NumOfKeys` (+ (`self.NumOfKeys`) 1)))
            (:`Collectable`
              (set `self.Collection` (+ (`self.Collection`) 1)))
            (:`Blank`
              (bind _asbp_abstract_myst_2 (cast `/Game/MapMysteries/BP_AbstractMyst` (`self.GetParentActor` HitActor)))
              (`/Engine/EditorBlueprintResources/StandardMacros.IsValid` _asbp_abstract_myst_2
                (:`Is Valid`
                  (`/Game/MapMysteries/BP_AbstractMyst.StartSpecificLogic` _asbp_abstract_myst_2 HitActor))))))
        (:`then_1`
          (`/Engine/EditorBlueprintResources/StandardMacros.IsValid` _asbp_switcheble_object
            (:`Is Valid`
              (`/Game/MapMeshes/BP_SwitchebleObject.StartLogic` _asbp_switcheble_object))))))))

(fn `StaminaUse`
  (params (IsUseStamina :type Boolean))
  (bind _regenspeed (`self.RegenSpeed`))
  (set `self.Stamina` (`KismetMathLibrary.FInterpTo_Constant` (`self.Stamina`) (select `bool` IsUseStamina :`false` (`self.MaxStamina`)) (`GameplayStatics.GetWorldDeltaSeconds`) (select `bool` IsUseStamina :`false` (/ _regenspeed 2.0) :`true` _regenspeed)))
  (if (<= (`self.Stamina`) 1.0)
    (if (not (`self.IsCrouch`))
      (`self.StopRun`))))

(fn `UserConstructionScript`
  (`SceneComponent.K2_AttachToComponent` (`self.ClockShowOff`) (`self.ArmShowOff`) "Clock" "SnapToTarget" "KeepRelative" "SnapToTarget" true)
  (`SceneComponent.K2_AttachToComponent` (`self.Clock`) (`self.Arm`) "Clock" "SnapToTarget" "KeepRelative" "SnapToTarget" true))