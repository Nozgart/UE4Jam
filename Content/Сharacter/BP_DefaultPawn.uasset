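; BP_DefaultPawn is a pawn that turns part of itself to face the mouse cursor.
; Every Tick it deprojects the cursor into the world, using the camera-to-mesh distance as depth along the ray.
; It then sets the Scene component's relative rotation to look at that point at the actor's own height, keeping the turn horizontal.
; An unconnected variant that rotates the whole actor is left in the graph.
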(event `self.ReceiveTick`
  (params (DeltaSeconds :type "Float (single-precision)"))
  (bind _returnvalue (`self.K2_GetActorLocation`))
  (bind (_worldlocation _worlddirection) (`PlayerController.DeprojectMousePositionToWorld` (`GameplayStatics.GetPlayerController` 0)))
  (`SceneComponent.K2_SetRelativeRotation` (`self.Scene`) (`KismetMathLibrary.FindLookAtRotation` _returnvalue (`KismetMathLibrary.MakeVector` (.x (+ _worldlocation (* _worlddirection (`KismetMathLibrary.VSize` (- (`SceneComponent.K2_GetComponentLocation` (`self.StaticMesh`)) (`SceneComponent.K2_GetComponentLocation` (`self.Camera`))))))) (.y (+ _worldlocation (* _worlddirection (`KismetMathLibrary.VSize` (- (`SceneComponent.K2_GetComponentLocation` (`self.StaticMesh`)) (`SceneComponent.K2_GetComponentLocation` (`self.Camera`))))))) (.z _returnvalue))) false false))

(fn `UserConstructionScript`)