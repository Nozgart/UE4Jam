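; BP_JobaPlayerController is the player controller that handles pausing for the Joba character.
; The ExitButton input calls a PauseGame event, which casts the controlled pawn to BP_JobaCharacter and toggles the paused state.
; Each toggle also sets mouse cursor visibility and tells the character's UiMain widget to enable or disable its pause display.
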(event `PauseGame`
  (bind _asbp_joba_character (cast `/Game/Сharacter/BP_JobaCharacter` (`self.K2_GetPawn`)))
  (if (`GameplayStatics.IsGamePaused`)
    (bind _uimain (`/Game/Сharacter/BP_JobaCharacter.UiMain` _asbp_joba_character))
    (`/Game/Widgets/MainUi.PauseDisabled` _uimain)
    (set `self.bShowMouseCursor` false)
    (`GameplayStatics.SetGamePaused` false)
    (else
      (`/Game/Widgets/MainUi.PauseEnabled` _uimain)
      (set `self.bShowMouseCursor` true)
      (`GameplayStatics.SetGamePaused` true))))

(event `InputAction|ExitButton` :paused true
  (params (Key :type "Key Structure"))
  (:`Pressed`
    (`self.PauseGame`)))

(fn `UserConstructionScript`)